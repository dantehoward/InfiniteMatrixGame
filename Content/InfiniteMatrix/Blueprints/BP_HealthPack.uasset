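; BP_HealthPack is a health pickup actor that heals the player on overlap.
; An overlapping actor that casts to BP_Player has IncreaseHealth called on it; the pack is not destroyed by that overlap.
; Each tick spins the mesh on yaw at RotateSpeed and destroys the actor once its age reaches DespawnTime.
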(event EventTick
  (params (DeltaSeconds :type Float%20%28single-precision%29))
  (Utilities|FlowControl|Sequence
    (:then_0
      (Transformation|AddLocalRotation (Variables|Default|GetHealthPackMesh) (Math|Rotator|MakeRotator 0.0 0.0 (* DeltaSeconds (Variables|Default|GetRotateSpeed))) false false))
    (:then_1
      (if (>= (Actor|GetGameTimeSinceCreation) (Variables|Default|GetDespawnTime))
        (Actor|DestroyActor)))))

(event Collision|EventActorBeginOverlap
  (params (OtherActor :type Actor%20Object%20Reference))
  (bind _asbp_player (Utilities|Casting|CastToBP_Player OtherActor))
  (Default|IncreaseHealth _asbp_player))

(fn ConstructionScript)